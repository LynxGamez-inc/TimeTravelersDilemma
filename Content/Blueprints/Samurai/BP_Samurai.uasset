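; BP_Samurai is an interactable Samurai character that displays a name label taken from CharacterName, set in the construction script.
; SetInteractableState shows or hides that label.
; A capsule overlap with BP_MainCharacter registers the Samurai as that character's OverlappingItem, with no matching end-overlap handler to clear it.
; Interact only stores the instigator and prints a debug message, as the overlap handler also does.
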(event `InteractInterface.SetInteractableState`
  (params (bCanShowInteract :type Boolean))
  (if bCanShowInteract
    (`SceneComponent.SetVisibility` (`self.Txt_CharacterName`) true false)
    (else
      (`SceneComponent.SetVisibility` (`self.Txt_CharacterName`) false false))))

(event `self.CapsuleComponent.OnComponentBeginOverlap`
  (params (OverlappedComponent :type "PrimitiveComponent Object Reference") (OtherActor :type "Actor Object Reference") (OtherComp :type "PrimitiveComponent Object Reference") (OtherBodyIndex :type Integer) (bFromSweep :type Boolean) (SweepResult :type "HitResult Structure (by ref)"))
  ;[1 1 1] fill overlapping Item in Main Character
  (bind _asbp_main_character (cast `/Game/Blueprints/Characters/BP_MainCharacter` OtherActor))
  (set `self.As BP Main Character_0` _asbp_main_character)
  (bind _output_get (set `self.BPSamuraiObj` self))
  (set `MainCharacter.OverlappingItem` _output_get (`self.As BP Main Character_0`))
  (`KismetSystemLibrary.PrintString` "overlap function in BPSamurai " true true (struct :`G` 0.923001 :`B` 1.0 :`A` 1.0)))

(event `InteractInterface.Interact`
  (params (InstigatorActor :type "Actor Object Reference"))
  (set `self.InteractInstigator` InstigatorActor)
  (`KismetSystemLibrary.PrintString` "Interact function in BPSamurai Successful!" true true (struct :`R` 1.0 :`B` 0.069834 :`A` 1.0)))

(fn `UserConstructionScript`
  (`TextRenderComponent.K2_SetText` (`self.Txt_CharacterName`) (`self.CharacterName`)))