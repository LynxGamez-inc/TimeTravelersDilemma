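; Letter item Blueprint that shows a typewriter-style letter when a lantern-equipped MainCharacter overlaps its box collision.
; The overlap disables the character's input mapping context, then reveals the WB_LetterWidget after a short delay.
; A looping timer at TypeSpeed appends InputText one character at a time to the widget.
; After the last character and a pause, it clears the timer, hides the widget and restores input.
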(event `self.ReceiveBeginPlay`
  (bind _returnvalue (`WidgetComponent.GetWidget` (`self.LetterWidget`)))
  (`UserWidget.AddToViewport` _returnvalue 0)
  (`Widget.SetVisibility` _returnvalue "Hidden")
  (bind _aswb_letter_widget (cast `/Game/Blueprints/Items/Letter/WB_LetterWidget` (`WidgetComponent.GetWidget` (`self.LetterWidget`))))
  (set `self.As WB Letter Widget` _aswb_letter_widget))

(event `self.BoxCollision.OnComponentBeginOverlap`
  (params (OverlappedComponent :type "PrimitiveComponent Object Reference") (OtherActor :type "Actor Object Reference") (OtherComp :type "PrimitiveComponent Object Reference") (OtherBodyIndex :type Integer) (bFromSweep :type Boolean) (SweepResult :type "HitResult Structure (by ref)"))
  (bind _asmain_character (cast `MainCharacter` OtherActor))
  (if (`MainCharacter.bIsLanternEquipped` _asmain_character)
    (`MainCharacter.DisableIMC` _asmain_character)
    (`KismetSystemLibrary.Delay` 1.0)
    (`Widget.SetVisibility` (`WidgetComponent.GetWidget` (`self.LetterWidget`)) "Visible")
    (bind _as_wb_letter_widget (`self.As WB Letter Widget`)
      (:`then`
        (`KismetSystemLibrary.Delay` 1.0)
        (bind _returnvalue (`KismetSystemLibrary.K2_SetTimerDelegate` (delegate `StartLoop`) (`self.TypeSpeed`) true)))
      (:`else`))))

(event `StartLoop`
  (bind _output_get (set `self.DisplayedText` (`KismetStringLibrary.Concat_StrStr` (`self.DisplayedText`) (`|GetArrayItem` (`KismetStringLibrary.GetCharacterArrayFromString` (`self.InputText`)) (`self.Index`)))))
  (`/Game/Blueprints/Items/Letter/WB_LetterWidget.Start Typing Letter` (stale `self.BoxCollision.OnComponentBeginOverlap` _as_wb_letter_widget) (`KismetTextLibrary.Conv_StringToText` _output_get))
  (bind _result (`/Engine/EditorBlueprintResources/StandardMacros.IncrementInt` (`self.Index`))
    (:`  `
      (if (== _result (`KismetArrayLibrary.Array_Length` (`KismetStringLibrary.GetCharacterArrayFromString` (`self.InputText`))))
        (`KismetSystemLibrary.Delay` 3.0)
        (`KismetSystemLibrary.K2_ClearAndInvalidateTimerHandle` (stale `self.BoxCollision.OnComponentBeginOverlap` _returnvalue))
        (`Widget.SetVisibility` (`WidgetComponent.GetWidget` (`self.LetterWidget`)) "Hidden")
        (`MainCharacter.EnableIMC` (stale `self.BoxCollision.OnComponentBeginOverlap` _asmain_character))))))

(fn `UserConstructionScript`)